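; Spline actor that draws a colored path through a supplied array of points, apparently as a support visual for player NPCs.
; AddSplinePoint builds the spline, using forward, backward and downward traces to insert height-adjusted points around blocking geometry.
; UpdateSpline sets point types from VisualFormPath, and AddSplineMesh creates scaled spline mesh segments using the dynamic material from AddMaterial, recording them in OldsMeshesPath.
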(event Collision|EventActorBeginOverlap
  (params (OtherActor :type Actor%20Object%20Reference)))

(event EventTick
  (params (DeltaSeconds :type Float%20%28single-precision%29)))

(fn ConstructionScript)

(fn CreateSplineMesh
  (params (Material :type Material%20Interface%20Object%20Reference) (CurrentPoint :type Integer) (TotalPoint :type Integer) (Spline :type Spline%20Component%20Object%20Reference) (VisualFormPath :type E_VisualFormPath%20Enum))
  (LocalVariables|SetL_Material Material)
  (LocalVariables|SetL_Spline Spline)
  (LocalVariables|SetL_CurrentPath CurrentPoint)
  (LocalVariables|SetL_TotalPoint TotalPoint)
  (switch Utilities|FlowControl|Switch|SwitchonE_VisualFormPath VisualFormPath
    (:NewEnumerator0
      (bind _returnvalue (AddComponent|AddSplineMeshComponent true :!label _label))
      (LocalVariables|SetL_SM _returnvalue))
    (:NewEnumerator1
      (if (== (LocalVariables|GetL_TotalPoint) 0)
        (bind _returnvalue_2 (AddComponent|AddSplineMeshComponent true))
        (LocalVariables|SetL_SM _returnvalue_2)
        (elif (== (LocalVariables|GetL_CurrentPath) 0)
          (bind _returnvalue_3 (AddComponent|AddSplineMeshComponent true))
          (LocalVariables|SetL_SM _returnvalue_3)
          (elif (== (LocalVariables|GetL_CurrentPath) (LocalVariables|GetL_TotalPoint))
            (bind _returnvalue_4 (AddComponent|AddSplineMeshComponent true))
            (LocalVariables|SetL_SM _returnvalue_4)
            (else
              (bind _returnvalue_5 (AddComponent|AddSplineMeshComponent true))
              (LocalVariables|SetL_SM _returnvalue_5))))))
    (:NewEnumerator2
      (goto _label)))
  (Rendering|Material|SetMaterial (LocalVariables|GetL_SM) 0 (LocalVariables|GetL_Material))
  (return (LocalVariables|GetL_SM)))

(fn AddSplinePoint
  (params (ArrayPoint :type Array%20of%20Vectors))
  (bind _spline (Variables|Default|GetSpline))
  (LocalVariables|SetL_ArrayPoint ArrayPoint)
  (for (_array_element _array_index) (LocalVariables|GetL_ArrayPoint)
    (bind _output_get (LocalVariables|SetL_CurrentPathIndex _array_index))
    (LocalVariables|SetL_CurrentPathLocation _array_element)
    (if (== _output_get (Utilities|Array|LastIndex (LocalVariables|GetL_ArrayPoint)))
      (Spline|AddSplinePoint (Variables|Default|GetSpline) (|CalculateLocationEndPoint_2) "World" false)
      (if (< (Math|Vector|VectorLength (- (Utilities|Array|Get(acopy) (LocalVariables|GetL_ArrayPoint) (Utilities|Array|LastIndex (LocalVariables|GetL_ArrayPoint))) (Utilities|Array|Get(acopy) (LocalVariables|GetL_ArrayPoint) (- (Utilities|Array|LastIndex (LocalVariables|GetL_ArrayPoint)) 1)))) 5e+01)
        (Spline|RemoveSplinePoint _spline (- (Spline|GetNumberOfSplinePoints _spline) 1) false))
      (else
        (Spline|AddSplinePoint (Variables|Default|GetSpline) (|CalculatePointLocation_2) "World" false)
        (|CalculateAltPathOverBlock_2)))))

(fn AddSplineMesh
  (bind _spline (Variables|Default|GetSpline))
  (bind _scalepath (Variables|Default|GetScalePath))
  (bind _spline_2 (Variables|Default|GetSpline))
  (bind _returnvalue (Spline|GetNumberOfSplinePoints _spline))
  (bind _returnvalue_2 (Math|Vector2D|MakeVector2D _scalepath _scalepath))
  (bind _returnvalue_3 (- _returnvalue 1))
  (for _index (range 0 _returnvalue_3)
    (LocalVariables|SetL_SplineIndex _index)
    (bind _smc (CallFunction|CreateSplineMesh (Variables|Default|GetD_Material) (LocalVariables|GetL_SplineIndex) _returnvalue_3 (Variables|Default|GetSpline) (Variables|Default|GetVisualFormPath)))
    (bind _output_get (Variables|Default|SetL_SMC _smc))
    (Utilities|Array|Add (Variables|Default|GetOldsMeshesPath) _output_get)
    (SplineMesh|SetEndScale (Variables|Default|GetL_SMC) _returnvalue_2 false :!class /Script/Engine.SplineMeshComponent)
    (SplineMesh|SetStartScale (Variables|Default|GetL_SMC) _returnvalue_2 false :!class /Script/Engine.SplineMeshComponent)
    (SplineMesh|SetStartandEnd (Variables|Default|GetL_SMC) (.Location (Spline|GetLocationandTangentatSplinePoint _spline_2 (LocalVariables|GetL_SplineIndex) "World")) (.Tangent (Spline|GetLocationandTangentatSplinePoint _spline_2 (LocalVariables|GetL_SplineIndex) "World")) (.Location (Spline|GetLocationandTangentatSplinePoint _spline_2 (+ (LocalVariables|GetL_SplineIndex) 1) "World")) (Utilities|Select :Index (Variables|Default|GetVisualFormPath) :NewEnumerator0 (.Tangent (Spline|GetLocationandTangentatSplinePoint _spline_2 (LocalVariables|GetL_SplineIndex) "World")) :NewEnumerator1 (Math|Vector|ClampVectorSize (.Tangent (Spline|GetLocationandTangentatSplinePoint _spline_2 (+ (LocalVariables|GetL_SplineIndex) 1) "World")) 0.0 1e+02) :NewEnumerator2 (.Tangent (Spline|GetLocationandTangentatSplinePoint _spline_2 (+ (LocalVariables|GetL_SplineIndex) 1) "World"))) true :!class /Script/Engine.SplineMeshComponent))
  (return (Variables|Default|GetL_SMC)))

(fn AddMaterial
  (params (Parent :type Material%20Interface%20Object%20Reference) (Value :type Linear%20Color%20Structure))
  (bind _returnvalue (Rendering|Material|CreateDynamicMaterialInstance Parent :!class /Script/Engine.KismetMaterialLibrary))
  (bind _output_get (Variables|Default|SetD_Material _returnvalue))
  (Rendering|Material|SetVectorParameterValue _output_get "Color" Value :!class /Script/Engine.MaterialInstanceDynamic))

(fn UpdateSpline
  (for _index (range 0 (Spline|GetNumberOfSplinePoints (Variables|Default|GetSpline)))
    (Spline|SetSplinePointType (Variables|Default|GetSpline) _index (Utilities|Select :Index (Variables|Default|GetVisualFormPath) :NewEnumerator0 "Linear" :NewEnumerator1 "CurveClamped" :NewEnumerator2 "CurveClamped") false))
  (Spline|UpdateSpline (Variables|Default|GetSpline))
  (return))