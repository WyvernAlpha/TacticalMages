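; BP_Correct_SM_OnMap is a support actor that snaps placed actors' X and Y positions to a grid, keeping their Z.
; One function processes every actor of the classes in ActorsForCorrect; the other processes all StaticMeshActors, then destroys the tool actor.
; Anything tagged "Don't Correct" is skipped, checked on the mesh component for StaticMeshActors and on the actor otherwise.
; The construction script sets that tag name and an instruction string.
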(event EventBeginPlay)

(event Collision|EventActorBeginOverlap
  (params (OtherActor :type Actor%20Object%20Reference)))

(event EventTick
  (params (DeltaSeconds :type Float%20%28single-precision%29)))

(fn ConstructionScript
  (Variables|Settings|SetInstruction:%20 "You need to add a Tag to your Static Meshes or Actors. 
If you do not want to adjust them")
  (Variables|Settings|SetTagName "Don't Correct"))

(fn RunCorrectPositionSM
  (for _array_element (Variables|Settings|GetActorsForCorrect)
    (bind _outactors (Actor|GetAllActorsOfClass _array_element))
    (for _array_element_2 _outactors
      (if (CallFunction|CheckforTeg _array_element_2)
        (Transformation|SetActorLocation _array_element_2 (CallFunction|CalculateGrid _array_element_2) false true)))))

(fn RunCorrectPositionSMandDestroySelf
  (bind _outactors (Actor|GetAllActorsOfClass "/Script/Engine.StaticMeshActor"))
  (for _array_element _outactors
    (if (CallFunction|CheckforTeg _array_element)
      (Transformation|SetActorLocation _array_element (CallFunction|CalculateGrid _array_element) false true)))
  (Actor|DestroyActor))

(fn CheckforTeg
  (params (Actor :type Actor%20Object%20Reference))
  (bind _tagname (Variables|Settings|GetTagName))
  (bind _asstatic_mesh_actor (Utilities|Casting|CastToStaticMeshActor Actor))
  (return (not (select (Utilities|IsValid _asstatic_mesh_actor) (Components|ComponentHasTag (Variables|/Script/Engine.StaticMeshActor|GetStaticMeshComponent _asstatic_mesh_actor) _tagname) (Actor|ActorHasTag Actor _tagname)))))

(fn CalculateGrid
  (params (Actor :type Actor%20Object%20Reference))
  (bind _returnvalue (Transformation|GetActorLocation Actor))
  (bind _gridsize (Variables|Default|GetGridSize))
  (return (Math|Vector|MakeVector (Math|Float|SnapToGrid(Float) (.x _returnvalue) _gridsize) (Math|Float|SnapToGrid(Float) (.y _returnvalue) _gridsize) (.z _returnvalue))))