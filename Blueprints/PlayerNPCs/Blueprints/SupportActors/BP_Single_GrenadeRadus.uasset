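; BP_Single_GrenadeRadus is a player-NPC support actor that, judging by its name, marks a grenade's radius with a cylinder mesh and a floor decal.
; On BeginPlay, SetMaterialAndForm applies configurable materials to the cylinder and decal.
; When NewFloorForm is valid, it also swaps the Cylinder and FloorCylinder meshes.
; The ClearPointDestination event calls ResetParameter, which is an empty stub.
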(event Custom|ClearPointDestination
  (CallFunction|ResetParameter))

(event EventBeginPlay
  (CallFunction|SetMaterialandForm))

(event Collision|EventActorBeginOverlap
  (params (OtherActor :type Actor%20Object%20Reference)))

(event EventTick
  (params (DeltaSeconds :type Float%20%28single-precision%29)))

(fn ConstructionScript)

(fn SetMaterialandForm
  (bind _newfloorform (Variables|Default|GetNewFloorForm))
  (Rendering|Material|SetMaterial (Variables|Default|GetCylinder) 0 (Variables|Default|GetMaterial))
  (Rendering|Components|Decal|SetDecalMaterial (Variables|Default|GetDecal) (Variables|Default|GetFloorMaterial))
  (Utilities|IsValid _newfloorform
    (:Is%20Valid
      (Components|StaticMesh|SetStaticMesh (Variables|Default|GetCylinder) _newfloorform)
      (Components|StaticMesh|SetStaticMesh (Variables|Default|GetFloorCylinder) (Variables|Default|GetFloor)))))

(fn ResetParameter)