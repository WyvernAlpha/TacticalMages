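; A thrown grenade actor that explodes shortly after its projectile movement nearly comes to rest, dealing radial damage.
; Tick watches the velocity, then disables itself, turns on physics for the detection sphere and starts a short fuse delay.
; The explosion fires a detonation dispatcher, spawns a particle effect, applies full damage credited to the first player controller, draws a debug sphere and destroys the actor.
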(event Custom|Event_Explosion
  (bind _returnvalue (Transformation|GetActorLocation))
  (bind _damageradius (Variables|Settings|GetDamageRadius))
  (Default|CallDGrenadeWasDetonated)
  (Effects|SpawnEmitteratLocation 0 (Transformation|GetActorLocation)) ; Grenade Visula Effect
  (Game|Damage|ApplyRadialDamage (Variables|Settings|GetGrenadeDamage) _returnvalue _damageradius 0 0 self (Game|GetPlayerController 0) true "ECC_Pawn") ; Apply damage from Grenade
  (Rendering|Debug|DrawDebugSphere _returnvalue _damageradius 12 "(R=1.000000,G=1.000000,B=1.000000,A=1.000000)" 2.0 2.0) ; No need after add Visual Effect explosive
  (EventDispatchers|UnbindallEventsfromDGrenadeWasDetonated)
  (Actor|DestroyActor))

(event EventBeginPlay)

(event Collision|EventActorBeginOverlap
  (params (OtherActor :type Actor%20Object%20Reference)))

(event EventTick
  (params (DeltaSeconds :type Float%20%28single-precision%29))
  (if (< (Math|Vector|VectorLength (Variables|/Script/Engine.MovementComponent|GetVelocity (Variables|Default|GetProjectileMovement))) 1e+01)
    (Actor|Tick|SetActorTickEnabled false)
    ;[1 1 1] Disable this node if you want a static Grenade
    (Physics|SetSimulatePhysics (Variables|Default|GetDetectSphere) true) ; Disable this node if you want a static Grenade
    (Utilities|FlowControl|Delay 1.0)
    (CallFunction|EventExplosion)))

(fn ConstructionScript)