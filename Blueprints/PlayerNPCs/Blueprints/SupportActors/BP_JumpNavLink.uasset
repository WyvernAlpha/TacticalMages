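; Nav link actor that moves AI characters across gaps and obstacles with jump, vault, slide or climb moves.
; On reaching the link, Tick turns the character toward the destination, then flags pick montage-driven moves, gated by a minimum-height check.
; Plain jumps and slide-overs launch with a computed ballistic velocity; slide-down uses MoveComponentTo.
; Climbing uses Flying mode and a widened capsule, with a timer restoring walking once speed picks up.
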(event Custom|Event_Jump
  (if (not (CallFunction|Checks))
    (Utilities|JumpOverAnimation)
    (Utilities|SlideOverAnimation)
    (Utilities|SlideDownAnimation)
    (Utilities|ClimbUpAnimation
      (:else
        (CallFunction|JumpLogic)))))

(event Custom|EnableMovementMode
  (bind _currentcharacter (Variables|Default|GetCurrentCharacter))
  (bind _charactermovement (Variables|/Script/Engine.Character|GetCharacterMovement _currentcharacter))
  (if (> (Math|Vector|VectorLength (Variables|/Script/Engine.MovementComponent|GetVelocity _charactermovement)) 4e+02)
    (Pawn|Components|CharacterMovement|SetMovementMode _charactermovement "MOVE_Walking" 0)
    (Components|Capsule|SetCapsuleRadius (Variables|/Script/Engine.Character|GetCapsuleComponent (Variables|Default|GetCurrentCharacter)) (/ (Variables|/Script/Engine.CapsuleComponent|GetCapsuleRadius (Variables|/Script/Engine.Character|GetCapsuleComponent (Variables|Default|GetCurrentCharacter))) 1.5) true)
    (Utilities|Time|ClearandInvalidateTimerbyHandle (Variables|Default|GetTimer))
    (Variables|/Script/Engine.CharacterMovementComponent|SetMaxWalkSpeed (Variables|/Script/Engine.Character|GetCharacterMovement (Variables|Default|GetCurrentCharacter)) 6e+02)))

(event EventBeginPlay)

(event Collision|EventActorBeginOverlap
  (params (OtherActor :type Actor%20Object%20Reference)))

(event EventTick
  (params (DeltaSeconds :type Float%20%28single-precision%29))
  (bind (_rotation _successful) (CallFunction|CalculateAxisRotation))
  (if (Variables|Default|GetEnableTickLogic)
    (Transformation|SetActorRotation (Variables|Default|GetCurrentCharacter) _rotation)
    (if _successful
      (Variables|Default|SetEnableTickLogic false)
      (CallFunction|EventJump))))

(event EventSmartLinkReached
  (params (Agent :type Actor%20Object%20Reference) (Destination :type Vector%20%28by%20ref%29))
  (Variables|Default|SetPointDestination Destination)
  (Variables|Default|SetCurrentCharacter (.AsCharacter (Utilities|Casting|CastToCharacter Agent)))
  (Variables|Default|SetEnableTickLogic true)
  (if (not (CallFunction|Checks))
    (Variables|/Script/Engine.CharacterMovementComponent|SetMaxWalkSpeed (Variables|/Script/Engine.Character|GetCharacterMovement (Variables|Default|GetCurrentCharacter)) 5e+01)))

(fn ConstructionScript
  (bind _output_get (Variables|Default|SetMinHeight (.z (Variables|Default|GetMinHeightDestination)))))

(fn CalculateVelocity
  (params (StartLocation :type Vector) (EndLocation :type Vector) (Duration :type Float%20%28single-precision%29))
  (bind (_x _y _z) (Math|Vector|BreakVector StartLocation))
  (bind (_x_2 _y_2 _z_2) (Math|Vector|BreakVector EndLocation))
  (Variables|Default|SetDuration Duration)
  (return (Math|Vector|MakeVector (/ (- _x_2 _x) (Variables|Default|GetDuration)) (/ (- _y_2 _y) (Variables|Default|GetDuration)) (/ (- _z_2 (+ _z (* (Math|Float|Square (Variables|Default|GetDuration)) -0.5 982.0))) (Variables|Default|GetDuration)))))

(fn CalculateAxisRotation
  (bind _returnvalue (Utilities|Time|GetWorldDeltaSeconds))
  (bind _currentcharacter (Variables|Default|GetCurrentCharacter))
  (bind _currentcharacter_2 (Variables|Default|GetCurrentCharacter))
  (bind _pointdestination (Variables|Default|GetPointDestination))
  (bind _returnvalue_2 (Transformation|GetActorRotation _currentcharacter_2))
  (bind _returnvalue_3 (Transformation|GetActorLocation _currentcharacter))
  (bind _returnvalue_4 (Math|Rotator|MakeRotator (.roll _returnvalue_2) (.pitch _returnvalue_2) (.yaw _returnvalue_2)))
  (bind _returnvalue_5 (Math|Rotator|FindLookatRotation _returnvalue_3 _pointdestination))
  (bind _yaw (Math|Rotator|BreakRotator _returnvalue_5))
  (bind _returnvalue_6 (Math|Rotator|MakeRotator (.roll _returnvalue_2) (.pitch _returnvalue_2) _yaw))
  (bind _returnvalue_7 (Math|Interpolation|RInterpTo _returnvalue_4 _returnvalue_6 _returnvalue 5.0))
  (return _returnvalue_7 (Math|Rotator|Equal(Rotator) _returnvalue_7 (Transformation|GetActorRotation (Variables|Default|GetCurrentCharacter)) 0.1)))

(fn JumpLogic
  (bind _velocity (CallFunction|CalculateVelocity (Transformation|GetActorLocation (Variables|Default|GetCurrentCharacter)) (Variables|Default|GetPointDestination) (Variables|Default|GetDuration))) ; JumpDown
  (Character|LaunchCharacter (Variables|Default|GetCurrentCharacter) _velocity true true)
  (Variables|/Script/Engine.CharacterMovementComponent|SetMaxWalkSpeed (Variables|/Script/Engine.Character|GetCharacterMovement (Variables|Default|GetCurrentCharacter)) 6e+02))

(fn Checks
  (bind _currentcharacter (Variables|Default|GetCurrentCharacter))
  (bind _capsulecomponent (Variables|/Script/Engine.Character|GetCapsuleComponent _currentcharacter))
  (return (and (< (- (.z (Variables|Default|GetPointDestination)) (- (.z (Transformation|GetWorldLocation _capsulecomponent)) (Variables|/Script/Engine.CapsuleComponent|GetCapsuleHalfHeight _capsulecomponent))) (Variables|Default|GetMinHeight)) (Math|Boolean|ORBoolean (Variables|Default|GetJumpOver?) (Variables|Default|GetSlideOver?) (Variables|Default|GetSlideDown?) (Variables|Default|GetClimbUp?)))))