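; BP_Single_TestNPC_Child is a child NPC Blueprint serving as an example of passing parameters to an Anim Blueprint when the skeletal mesh changes.
; It overrides SetFireDirectionandPitch, casts the mesh's anim instance to NPC_AnimBP, and feeds FireDirection and AimPitch to the parent implementation.
; The cast is the swap point for another Anim Blueprint; construction defers to the parent, and the other event stubs are disabled.
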(event EventBeginPlay
  (|CallParentFunction))

(event Collision|EventActorBeginOverlap
  (params (OtherActor :type Actor%20Object%20Reference)))

(event EventTick
  (params (DeltaSeconds :type Float%20%28single-precision%29))
  (|CallParentFunction DeltaSeconds))

(event EventSetFireDirectionandPitch
  (params (FireDirection :type Float%20%28single-precision%29) (AimPitch :type Float%20%28single-precision%29))
  ;[0.14 0 0] For example - how to transfer parameters to an animated blueprint when changing a skeletal mesh
  (bind _asnpc_anim_bp (Utilities|Casting|CastToNPC_AnimBP (CallFunction|AnimInstance))) ; You need to change this cast to your new Anim BP
  (|CallParentFunction (Variables|/Game/ATBS/Animations/PlayerNPCsAnimation/NPC_AnimBP.NPC_AnimBP_C|GetFireDirection _asnpc_anim_bp) (Variables|/Game/ATBS/Animations/PlayerNPCsAnimation/NPC_AnimBP.NPC_AnimBP_C|GetAimPitch _asnpc_anim_bp)))

(fn ConstructionScript
  (|CallParentFunction))

(fn AnimInstance
  (return (Components|SkeletalMesh|GetAnimInstance (Variables|Character|GetMesh))))