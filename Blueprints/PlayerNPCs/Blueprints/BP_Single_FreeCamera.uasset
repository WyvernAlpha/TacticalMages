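; Player free-camera actor for squad tactics that selects player NPCs by click, Tab or event and orders their moves.
; BeginPlay gathers the NPCs, assigns portraits and creates the HUD.
; Selection hands the NPC's path component to click-to-move, while right-click cancels or recenters according to MainState.
; CameraControlManager handles pan, zoom and rotation, with Tick following the NPC or enemy when focused; holding C makes the NPC ignore cursor traces.
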(event Custom|DefocusCamera
  ;[1 1 1] Shift camera to NPC
  (Variables|/Game/ATBS/Blueprints/PlayerNPCs/Blueprints/Components/BC_CameraControlManager.BC_CameraControlManager_C|SetCameraWasFocused? (Variables|Default|GetCameraControlManager) false))

(event Custom|Event_SelectCharacter
  (params (bIsSelectUse? :type Boolean) (CurrentNPC :type Actor%20Object%20Reference))
  (bind _hitactor (CallFunction|MouseLocation))
  (bind _currentpathcomponent (Variables|Default|GetCurrentPathComponent))
  ;[1 1 1] NPCs controls
  (bind _output_get (Variables|Default|SetIsUseSelect bIsSelectUse?))
  (if _output_get
    (if (not (Variables|Default|GetEndMatch))
      (if (!= _hitactor (Variables|Default|GetCurrentNPC))
        (Utilities|PreState)
        (Utilities|IsValid (Variables|Default|GetCurrentPathComponent)
          (:Is%20Valid
            (if (Utilities|ClassIsChildOf (Utilities|GetClass (select (Variables|Default|GetIsUseSelect) CurrentNPC _hitactor)) "/Game/ATBS/Blueprints/PlayerNPCs/Blueprints/BP_Single_TestNPC.BP_Single_TestNPC_C")
              (Default|DestroyPath (Variables|Default|GetCurrentPathComponent))
              (Default|DestroyZone (Variables|/Game/ATBS/Blueprints/PlayerNPCs/Blueprints/BP_Single_TestNPC.BP_Single_TestNPC_C|GetSingle_Movement_Area (Variables|Default|GetCurrentNPC)))
              (Class|Pawn|SetCanAffectNavigationGeneration (Variables|Default|GetCurrentNPC) true)
              (Rendering|SetVisibility (Variables|/Game/ATBS/Blueprints/PlayerNPCs/Blueprints/BP_Single_TestNPC.BP_Single_TestNPC_C|GetMarker (stale _currentnpc)) false false :!label _label)
              (bind _asbp_single_test_npc (Utilities|Casting|CastToBP_Single_TestNPC (select (Variables|Default|GetIsUseSelect) CurrentNPC (.HitActor (CallFunction|MouseLocation))) :!label _label_2))
              (bind _output_get_2 (Variables|Default|SetCurrentNPC _asbp_single_test_npc))
              (CallFunction|ChooseNPCandFocused _output_get_2)
              (Variables|Default|SetIsUseSelect false)
              (else
                (Utilities|IsValid _currentpathcomponent :!label _label_3
                  (:Is%20Valid
                    (if (Variables|/Game/ATBS/Blueprints/PlayerNPCs/Blueprints/Components/BC_Single_DrawPath.BC_Single_DrawPath_C|GetbCheckCanMove _currentpathcomponent)
                      (Default|UpdateWidget (Variables|Default|GetHUD))
                      (Variables|/Game/ATBS/Blueprints/PlayerNPCs/Blueprints/Components/BC_CameraControlManager.BC_CameraControlManager_C|SetCameraWasFocused? (Variables|Default|GetCameraControlManager) true)
                      (Default|DestroyZone (Variables|/Game/ATBS/Blueprints/PlayerNPCs/Blueprints/BP_Single_TestNPC.BP_Single_TestNPC_C|GetSingle_Movement_Area (Variables|Default|GetCurrentNPC)))
                      (Default|MoveNPCto (Variables|Default|GetCurrentNPC))
                      (Default|DontMoveEvent (Variables|Default|GetCurrentPathComponent) true)))))))
          (:Is%20Not%20Valid
            (if (Utilities|ClassIsChildOf (Utilities|GetClass (select (Variables|Default|GetIsUseSelect) CurrentNPC _hitactor)) "/Game/ATBS/Blueprints/PlayerNPCs/Blueprints/BP_Single_TestNPC.BP_Single_TestNPC_C")
              (bind _currentnpc (Variables|Default|GetCurrentNPC)
                (:then
                  (goto _label))
                (:else
                  (goto _label_2)))
              (else
                (goto _label_3)))))))))

(event Custom|ShiftCameraToNPC
  ;[1 1 1] Shift camera to NPC
  (Components|MoveComponentTo (VehicleSound|GetRootComponent) (Transformation|GetActorLocation (Variables|Default|GetCurrentNPC)) (Transformation|GetActorRotation) false false 0.3 false)
  (EventDispatchers|BindEventtoDMovementFinished (Variables|Default|GetCurrentPathComponent) (EventDispatchers|CreateEvent :!event Custom|DefocusCamera))
  (switch Utilities|FlowControl|Switch|SwitchonE_MainState (Variables|/Game/ATBS/Blueprints/PlayerNPCs/Blueprints/BP_Single_TestNPC.BP_Single_TestNPC_C|GetMainState (Variables|Default|GetCurrentNPC))
    (:NewEnumerator0
      _)
    (:NewEnumerator1
      _))
  (CallFunction|RestoreMovetState))

(event EventBeginPlay
  ;[0.9622 0 1] Create Master Hud Widget
  ; For example, add an image in the character selection panel
  (bind _outactors (Actor|GetAllActorsOfClass "/Game/ATBS/Blueprints/PlayerNPCs/Blueprints/BP_Single_TestNPC.BP_Single_TestNPC_C"))
  (Variables|Default|SetArrayAllPlayerNPCs _outactors)
  (CallFunction|SetupFaceImage)
  (bind _returnvalue (UserInterface|CreateWidget "/Game/ATBS/Blueprints/UI/W_Single_Hud.W_Single_Hud_C" (Game|GetPlayerController 0) self (Variables|Default|GetArrayAllPlayerNPCs)))
  (bind _output_get (Variables|Default|SetHUD _returnvalue))
  (UserInterface|Viewport|AddtoViewport _output_get 0))

(event Collision|EventActorBeginOverlap
  (params (OtherActor :type Actor%20Object%20Reference)))

(event EventTick
  (params (DeltaSeconds :type Float%20%28single-precision%29))
  (bind _enemynpc (Variables|Default|GetEnemyNPC))
  ;[1 1 1] Following Camera to NPC
  (if (Variables|/Game/ATBS/Blueprints/PlayerNPCs/Blueprints/Components/BC_CameraControlManager.BC_CameraControlManager_C|GetCameraWasFocused? (Variables|Default|GetCameraControlManager))
    (Transformation|SetActorLocation (Math|Interpolation|VInterpTo (Transformation|GetActorLocation) (Transformation|GetActorLocation (select (Utilities|IsValid _enemynpc) _enemynpc (Variables|Default|GetCurrentNPC))) (Utilities|Time|GetWorldDeltaSeconds) 1e+01) false false)))

(event Input|AxisEvents|InputAxisMoveForward
  (params (AxisValue :type Float%20%28single-precision%29))
  ;[1 1 1] Movement Camera
  (Default|MoveForward (Variables|Default|GetCameraControlManager) AxisValue))

(event Input|AxisEvents|InputAxisMoveRight
  (params (AxisValue :type Float%20%28single-precision%29))
  ;[1 1 1] Movement Camera
  (Default|MoveRight (Variables|Default|GetCameraControlManager) AxisValue))

(event Input|MouseEvents|MouseWheelAxis
  (params (AxisValue :type Float%20%28single-precision%29))
  ;[1 1 1] Camera Control
  (Default|CameraZoom (Variables|Default|GetCameraControlManager) AxisValue))

(event Input|MouseEvents|MouseY
  (params (AxisValue :type Float%20%28single-precision%29))
  ;[1 1 1] Camera Control
  (Default|CameraRotatePitch (Variables|Default|GetCameraControlManager) AxisValue))

(event Input|MouseEvents|MouseX
  (params (AxisValue :type Float%20%28single-precision%29))
  ;[1 1 1] Camera Control
  (Default|CameraRotateYaw (Variables|Default|GetCameraControlManager) AxisValue))

(event Input|KeyboardEvents|C
  (params (Key :type Key%20Structure :default "AnyKey"))
  ;[1 1 1] That can be helpful if you want to allow the player to make the NPC move just a bit.
  ; Or change the direction in which the NPC is looking
  (:Pressed
    (CallFunction|Enable1mOffset "ECR_Ignore"))
  (:Released
    (CallFunction|Enable1mOffset "ECR_Block")))

(event Input|MouseEvents|RightMouseButton
  (params (Key :type Key%20Structure :default "AnyKey"))
  (bind _cameracontrolmanager (Variables|Default|GetCameraControlManager))
  ;[1 1 1] Camera Control
  (:Pressed
    (Variables|/Game/ATBS/Blueprints/PlayerNPCs/Blueprints/Components/BC_CameraControlManager.BC_CameraControlManager_C|SetHoldRightMouseButton _cameracontrolmanager true))
  (:Released
    (Variables|/Game/ATBS/Blueprints/PlayerNPCs/Blueprints/Components/BC_CameraControlManager.BC_CameraControlManager_C|SetHoldRightMouseButton _cameracontrolmanager false)))

(event Input|MouseEvents|LeftMouseButton
  (params (Key :type Key%20Structure :default "AnyKey"))
  (bind _hitactor (CallFunction|MouseLocation))
  (bind _currentpathcomponent (Variables|Default|GetCurrentPathComponent))
  ;[1 1 1] NPCs controls
  (:Pressed
    (if (not (Variables|Default|GetEndMatch))
      (if (!= _hitactor (Variables|Default|GetCurrentNPC))
        (Utilities|PreState)
        (Utilities|IsValid (Variables|Default|GetCurrentPathComponent)
          (:Is%20Valid
            (if (Utilities|ClassIsChildOf (Utilities|GetClass (select (Variables|Default|GetIsUseSelect) (stale Custom|Event_SelectCharacter CurrentNPC) _hitactor)) "/Game/ATBS/Blueprints/PlayerNPCs/Blueprints/BP_Single_TestNPC.BP_Single_TestNPC_C")
              (Default|DestroyPath (Variables|Default|GetCurrentPathComponent))
              (Default|DestroyZone (Variables|/Game/ATBS/Blueprints/PlayerNPCs/Blueprints/BP_Single_TestNPC.BP_Single_TestNPC_C|GetSingle_Movement_Area (Variables|Default|GetCurrentNPC)))
              (Class|Pawn|SetCanAffectNavigationGeneration (Variables|Default|GetCurrentNPC) true)
              (Rendering|SetVisibility (Variables|/Game/ATBS/Blueprints/PlayerNPCs/Blueprints/BP_Single_TestNPC.BP_Single_TestNPC_C|GetMarker (stale _currentnpc)) false false :!label _label)
              (bind _asbp_single_test_npc (Utilities|Casting|CastToBP_Single_TestNPC (select (Variables|Default|GetIsUseSelect) (stale Custom|Event_SelectCharacter CurrentNPC) (.HitActor (CallFunction|MouseLocation))) :!label _label_2))
              (bind _output_get (Variables|Default|SetCurrentNPC _asbp_single_test_npc))
              (CallFunction|ChooseNPCandFocused _output_get)
              (Variables|Default|SetIsUseSelect false)
              (else
                (Utilities|IsValid _currentpathcomponent :!label _label_3
                  (:Is%20Valid
                    (if (Variables|/Game/ATBS/Blueprints/PlayerNPCs/Blueprints/Components/BC_Single_DrawPath.BC_Single_DrawPath_C|GetbCheckCanMove _currentpathcomponent)
                      (Default|UpdateWidget (Variables|Default|GetHUD))
                      (Variables|/Game/ATBS/Blueprints/PlayerNPCs/Blueprints/Components/BC_CameraControlManager.BC_CameraControlManager_C|SetCameraWasFocused? (Variables|Default|GetCameraControlManager) true)
                      (Default|DestroyZone (Variables|/Game/ATBS/Blueprints/PlayerNPCs/Blueprints/BP_Single_TestNPC.BP_Single_TestNPC_C|GetSingle_Movement_Area (Variables|Default|GetCurrentNPC)))
                      (Default|MoveNPCto (Variables|Default|GetCurrentNPC))
                      (Default|DontMoveEvent (Variables|Default|GetCurrentPathComponent) true)))))))
          (:Is%20Not%20Valid
            (if (Utilities|ClassIsChildOf (Utilities|GetClass (select (Variables|Default|GetIsUseSelect) (stale Custom|Event_SelectCharacter CurrentNPC) _hitactor)) "/Game/ATBS/Blueprints/PlayerNPCs/Blueprints/BP_Single_TestNPC.BP_Single_TestNPC_C")
              (bind _currentnpc (Variables|Default|GetCurrentNPC)
                (:then
                  (goto _label))
                (:else
                  (goto _label_2)))
              (else
                (goto _label_3)))))))))

(event Input|MouseEvents|RightMouseButton
  (params (Key :type Key%20Structure :default "AnyKey"))
  (bind _currentpathcomponent (Variables|Default|GetCurrentPathComponent))
  ;[1 1 1] NPCs controls
  (:Pressed
    (if (not (Variables|Default|GetEndMatch))
      (bind _currentnpc (Variables|Default|GetCurrentNPC)
        (:then
          (Components|Tick|SetComponentTickEnabled (Variables|/Game/ATBS/Blueprints/PlayerNPCs/Blueprints/BP_Single_TestNPC.BP_Single_TestNPC_C|GetSingle_ShowPath _currentnpc) false)
          (Utilities|FlowControl|Delay 0.2)
          (if (not (Variables|/Game/ATBS/Blueprints/PlayerNPCs/Blueprints/Components/BC_CameraControlManager.BC_CameraControlManager_C|GetHoldRightMouseButton (Variables|Default|GetCameraControlManager)))
            (switch Utilities|FlowControl|Switch|SwitchonE_MainState (Variables|/Game/ATBS/Blueprints/PlayerNPCs/Blueprints/BP_Single_TestNPC.BP_Single_TestNPC_C|GetMainState (Variables|Default|GetCurrentNPC))
              (:NewEnumerator0
                (CallFunction|ShiftCameratoNPC :!label _label))
              (:NewEnumerator1
                (goto _label))
              (:NewEnumerator3
                (CallFunction|RestoreMovetState :!label _label_2))
              (:NewEnumerator5
                (goto _label))
              (:NewEnumerator7
                (CallFunction|ShiftCameratoNPC)
                (goto _label_2)))
            (EventDispatchers|UnbindallEventsfromPressLMB)))
        (:else))))
  (:Released
    (Utilities|IsValid _currentpathcomponent
      (:Is%20Valid
        (Components|Tick|SetComponentTickEnabled _currentpathcomponent true)))))

(event Input|KeyboardEvents|Tab
  (params (Key :type Key%20Structure :default "AnyKey"))
  ;[1 1 1] NPCs controls
  (:Pressed
    (CallFunction|SelectCharacter true)))

(fn ConstructionScript)

(fn MouseLocation
  (bind _returnvalue (Game|GetPlayerController 0))
  (bind _hitresult (Game|Player|GetHitResultUnderCursorbyChannel _returnvalue "TraceTypeQuery2" true))
  (bind (_bblockinghit _binitialoverlap _time _location _impactpoint _normal _impactnormal _physmat _hitactor) (Collision|BreakHitResult _hitresult))
  (return _location _hitactor))

(fn ClearChosenNPC
  (bind _currentnpc (Variables|Default|GetCurrentNPC)
    (:then
      (Rendering|SetVisibility (Variables|/Game/ATBS/Blueprints/PlayerNPCs/Blueprints/BP_Single_TestNPC.BP_Single_TestNPC_C|GetMarker _currentnpc) false false))
    (:else
      _))
  (Variables|Default|SetCurrentPathComponent 0)
  (Variables|Default|SetCurrentNPC 0)
  (Variables|Default|SetEnemyNPC 0))

(fn ChooseNPCandFocused
  (params (CurrentNPCs :type Actor%20Object%20Reference))
  (bind _currentnpc (Variables|Default|GetCurrentNPC))
  (Utilities|IsValid CurrentNPCs
    (:Is%20Valid
      (Actor|SetOwner (Variables|Default|GetCurrentNPC) self)
      (Class|Pawn|SetCanAffectNavigationGeneration (Variables|Default|GetCurrentNPC) false)
      (Default|EventEnableOverview (Variables|Default|GetCurrentNPC))
      (Rendering|SetVisibility (Variables|/Game/ATBS/Blueprints/PlayerNPCs/Blueprints/BP_Single_TestNPC.BP_Single_TestNPC_C|GetMarker _currentnpc) true false)
      (Variables|Default|SetCurrentPathComponent (Variables|/Game/ATBS/Blueprints/PlayerNPCs/Blueprints/BP_Single_TestNPC.BP_Single_TestNPC_C|GetSingle_ShowPath _currentnpc))
      (Variables|/Game/ATBS/Blueprints/PlayerNPCs/Blueprints/BP_Single_TestNPC.BP_Single_TestNPC_C|SetHUD (Variables|Default|GetCurrentNPC) (Variables|Default|GetHUD))
      (Default|UpdateWidget (Variables|Default|GetHUD))
      (CallFunction|ShiftCameratoNPC)
      (Variables|Default|SetCurrentSelectCharacter (Utilities|Array|FindItem (Variables|Default|GetArrayAllPlayerNPCs) (Variables|Default|GetCurrentNPC)))
      (for _array_element (Variables|/Game/ATBS/Blueprints/UI/W_Single_Hud.W_Single_Hud_C|GetArrayButtonSelectCharacter (Variables|Default|GetHUD))
        (Class|Button|SetBackgroundColor (Variables|/Game/ATBS/Blueprints/UI/W_ButtonSelectCharacter.W_ButtonSelectCharacter_C|GetButton_203 _array_element) (Variables|/Game/ATBS/Blueprints/UI/W_ButtonSelectCharacter.W_ButtonSelectCharacter_C|GetColor _array_element)))
      (Class|Button|SetBackgroundColor (Variables|/Game/ATBS/Blueprints/UI/W_ButtonSelectCharacter.W_ButtonSelectCharacter_C|GetButton_203 (Utilities|Array|Get(acopy) (Variables|/Game/ATBS/Blueprints/UI/W_Single_Hud.W_Single_Hud_C|GetArrayButtonSelectCharacter (Variables|Default|GetHUD)) (Variables|Default|GetCurrentSelectCharacter))) "(R=0.755000,G=0.325485,B=0.000000,A=1.000000)")
      (return))))

(fn SetupFaceImage
  (for (_array_element _array_index) (Variables|Default|GetArrayAllPlayerNPCs)
    (bind _asbp_single_test_npc (Utilities|Casting|CastToBP_Single_TestNPC _array_element))
    (Variables|/Game/ATBS/Blueprints/PlayerNPCs/Blueprints/BP_Single_TestNPC.BP_Single_TestNPC_C|SetData _asbp_single_test_npc (Utilities|Struct|MakeST_PlayerNPCsData (.TeamID (Utilities|Struct|BreakST_PlayerNPCsData (Variables|/Game/ATBS/Blueprints/PlayerNPCs/Blueprints/BP_Single_TestNPC.BP_Single_TestNPC_C|GetData _asbp_single_test_npc))) (.Health (Utilities|Struct|BreakST_PlayerNPCsData (Variables|/Game/ATBS/Blueprints/PlayerNPCs/Blueprints/BP_Single_TestNPC.BP_Single_TestNPC_C|GetData _asbp_single_test_npc))) (Utilities|Array|Get(acopy) (Variables|Default|GetArrayImage) _array_index) (.WeaponAttackDistance (Utilities|Struct|BreakST_PlayerNPCsData (Variables|/Game/ATBS/Blueprints/PlayerNPCs/Blueprints/BP_Single_TestNPC.BP_Single_TestNPC_C|GetData _asbp_single_test_npc))) (.BeginItems (Utilities|Struct|BreakST_PlayerNPCsData (Variables|/Game/ATBS/Blueprints/PlayerNPCs/Blueprints/BP_Single_TestNPC.BP_Single_TestNPC_C|GetData _asbp_single_test_npc))))))
  (return))

(fn SelectCharacter
  (params (Increment? :type Boolean))
  (bind _arrayallplayernpcs (Variables|Default|GetArrayAllPlayerNPCs))
  (bind _currentnpc (Variables|Default|GetCurrentNPC))
  (Utilities|IsValid (Variables|Default|GetCurrentNPC)
    (:Is%20Valid
      (if (or (Default|CheckStateforTransit _currentnpc "NewEnumerator0") (Default|CheckStateforTransit _currentnpc "NewEnumerator5"))
        (if Increment?
          (Math|Integer|IncrementInt (Variables|Default|GetCurrentSelectCharacter)
            (:%20%20
              _))
          (elif (<= (Variables|Default|GetCurrentSelectCharacter) 0)
            (Variables|Default|SetCurrentSelectCharacter (Math|Integer|Max(Integer) (- (Utilities|Array|Length (Variables|Default|GetArrayAllPlayerNPCs)) 1)))
            (else
              (Math|Integer|DecrementInt (Variables|Default|GetCurrentSelectCharacter)
                (:%20%20
                  _)))))
        (Variables|Default|SetCurrentSelectCharacter (Math|Integer|%(Integer) (Variables|Default|GetCurrentSelectCharacter) (Utilities|Array|Length _arrayallplayernpcs)) :!label _label)
        (CallFunction|EventSelectCharacter true (Utilities|Array|Get(acopy) _arrayallplayernpcs (Math|Integer|%(Integer) (Variables|Default|GetCurrentSelectCharacter) (Utilities|Array|Length _arrayallplayernpcs))))))
    (:Is%20Not%20Valid
      (if Increment?
        (Math|Integer|IncrementInt (Variables|Default|GetCurrentSelectCharacter)
          (:%20%20
            (goto _label)))
        (elif (<= (Variables|Default|GetCurrentSelectCharacter) 0)
          (Variables|Default|SetCurrentSelectCharacter (Math|Integer|Max(Integer) (- (Utilities|Array|Length (Variables|Default|GetArrayAllPlayerNPCs)) 1)))
          (goto _label)
          (else
            (Math|Integer|DecrementInt (Variables|Default|GetCurrentSelectCharacter)
              (:%20%20
                (goto _label)))))))))

(fn RestoreMovetState
  (bind _canchangestate (Default|MainTransittoState (Variables|Default|GetCurrentNPC) "NewEnumerator4"))
  (if _canchangestate
    (Variables|Default|SetEnemyNPC 0)))

(fn Enable1mOffset
  (params (IgnoreSelf :type ECollisionResponse%20Enum))
  (bind _currentnpc (Variables|Default|GetCurrentNPC))
  (bind _returnvalue (VehicleSound|GetRootComponent _currentnpc))
  (bind _asprimitive_component (Utilities|Casting|CastToPrimitiveComponent _returnvalue))
  (Collision|SetCollisionResponsetoChannel _asprimitive_component "ECC_Camera" IgnoreSelf)
  (for _array_element (Components|GetChildrenComponents _returnvalue true)
    (bind _asprimitive_component_2 (Utilities|Casting|CastToPrimitiveComponent _array_element))
    (Collision|SetCollisionResponsetoChannel _asprimitive_component_2 "ECC_Camera" IgnoreSelf)))