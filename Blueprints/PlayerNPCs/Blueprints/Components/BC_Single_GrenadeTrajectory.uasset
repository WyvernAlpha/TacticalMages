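; Grenade-throw component that previews an arced trajectory and damage radius from the owning character toward the cursor or hovered hex cell.
; While enabled, Tick clamps the navmesh-resolved target to throw range and rebuilds spline meshes, end spheres and radius marker when it moves.
; VisualisePath predicts the projectile path, stepping the arc higher while it falls short.
; Event_CreatingTrajectory recalculates from the throw socket and stores launch velocity.
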(event Custom|Event_Create_Path
  (Variables|Hide|SetShowTrajectory? true))

(event Custom|DestroyPath
  (Variables|Hide|SetShowTrajectory? false)
  (CallFunction|ClearPath)
  (bind _endpointdestination (Variables|Hide|GetEndPointDestination)
    (:then
      (Actor|DestroyActor _endpointdestination))
    (:else)))

(event Custom|Event_ClearPath
  (Variables|Hide|SetShowTrajectory? false)
  (CallFunction|ClearPath)
  (bind _endpointdestination (Variables|Hide|GetEndPointDestination)
    (:then
      (Default|ClearPointDestination _endpointdestination))
    (:else)))

(event Custom|Event_StopDrawTrack
  (Variables|Hide|SetShowTrajectory? false))

(event Custom|Event_CreatingTrajectory
  (bind (_destinationpoint _beginpoint _l_arcparam1) (CallFunction|VisualisePath true))
  (bind _output_get (Variables|Hide|SetPointDestination _destinationpoint))
  (bind _outlaunchvelocity (Game|SuggestProjectileVelocityCustomArc _beginpoint _output_get 0.0 _l_arcparam1))
  (Variables|Hide|SetGrenadeVelocity _outlaunchvelocity)
  (CallFunction|UpdateCurrentSpline))

(event EventBeginPlay
  (bind _returnvalue (Components|GetOwner))
  (bind _trackcolor (Variables|TrackSettings|GetTrackColor))
  (bind (_r _g _b) (Utilities|Struct|BreakLinearColor _trackcolor))
  (Variables|PrivateVariable|SetOwnerController (AI|GetAIController _returnvalue))
  (bind _ascharacter (Utilities|Casting|CastToCharacter _returnvalue))
  (Variables|PrivateVariable|SetOwnerCharacter _ascharacter)
  (bind _returnvalue_2 (Rendering|Material|CreateDynamicMaterialInstance (Variables|TrackSettings|GetTrackMaterial) :!class /Script/Engine.KismetMaterialLibrary))
  (bind _output_get (Variables|Hide|SetD_Material _returnvalue_2))
  (Rendering|Material|SetVectorParameterValue _output_get "Color" (Utilities|Struct|MakeLinearColor _r _g _b 0.072982) :!class /Script/Engine.MaterialInstanceDynamic)
  (bind _returnvalue_3 (Rendering|Material|CreateDynamicMaterialInstance (Variables|TrackSettings|GetGrenadeRadiusMaterial) :!class /Script/Engine.KismetMaterialLibrary))
  (Variables|Hide|SetD_EndMaterial _returnvalue_3)
  (bind _returnvalue_4 (Rendering|Material|CreateDynamicMaterialInstance (Variables|Hide|GetGrenadeFloorMaterial) :!class /Script/Engine.KismetMaterialLibrary))
  (Variables|Hide|SetD_FloorMaterial _returnvalue_4))

(event EventTick
  (params (DeltaSeconds :type Float%20%28single-precision%29))
  (bind _selectormovement (Variables|TrackSettings|GetSelectorMovement))
  (bind _returnvalue (CallFunction|SwitchMovement _selectormovement))
  (if (Variables|Hide|GetShowTrajectory?)
    (Variables|Hide|SetCurrentCursorLocation _returnvalue)
    (bind _returnvalue_2 (Class|NavigationSystem|FindPathtoLocationSynchronously (Transformation|GetActorLocation (Components|GetOwner)) _returnvalue 0 "/Script/Engine.RecastFilter_UseDefaultArea"))
    (bind _output_get (Variables|Hide|SetPath (Variables|/Script/Engine.NavigationPath|GetPathPoints _returnvalue_2)))
    (if (not (Math|Vector|Equal(Vector) (Variables|Hide|GetLastCursorPosition) (Utilities|Array|Get(acopy) _output_get (Utilities|Array|LastIndex (Variables|/Script/Engine.NavigationPath|GetPathPoints _returnvalue_2))) (Variables|TrackSettings|GetAccuracyCursorRadius)))
      (if (not (Math|Vector|Equal(Vector) (Utilities|Array|Get(acopy) _output_get (Utilities|Array|LastIndex (Variables|/Script/Engine.NavigationPath|GetPathPoints _returnvalue_2))) "0, 0, 0" 0.0001))
        (if (Variables|PrivateVariable|GetTrackWasCreated)
          (CallFunction|ClearPath))
        (bind _destinationpoint (CallFunction|VisualisePath false))
        (CallFunction|EndDestination _destinationpoint)
        (CallFunction|UpdateCurrentSpline)
        (CallFunction|AddStaticMesh)
        (Variables|PrivateVariable|SetTrackWasCreated true)))))

(fn VisualisePath
  (params (NewParam :type Boolean))
  (bind _ownercharacter (Variables|PrivateVariable|GetOwnerCharacter))
  (bind _currentcursorlocation (Variables|Hide|GetCurrentCursorLocation))
  (bind _returnvalue (Transformation|GetActorLocation _ownercharacter))
  (LocalVariables|SetL_PathPoint (Variables|Hide|GetPath))
  (LocalVariables|SetL_BeginPoint (select NewParam (Transformation|GetSocketLocation (Variables|/Script/Engine.Character|GetMesh (Variables|PrivateVariable|GetOwnerCharacter)) (Variables|TrackSettings|GetSocketForThrow)) (Math|Vector|MakeVector (.X (Math|Vector|BreakVector (+ (+ _returnvalue (* (Math|Vector|GetRightVector (Math|Rotator|FindLookatRotation _returnvalue (Utilities|Array|Get(acopy) (LocalVariables|GetL_PathPoint) (Utilities|Array|LastIndex (LocalVariables|GetL_PathPoint))))) 3e+01)) (* (Math|Vector|GetForwardVector (Math|Rotator|FindLookatRotation _returnvalue (Utilities|Array|Get(acopy) (LocalVariables|GetL_PathPoint) (Utilities|Array|LastIndex (LocalVariables|GetL_PathPoint))))) -1e+01)))) (.Y (Math|Vector|BreakVector (+ (+ _returnvalue (* (Math|Vector|GetRightVector (Math|Rotator|FindLookatRotation _returnvalue (Utilities|Array|Get(acopy) (LocalVariables|GetL_PathPoint) (Utilities|Array|LastIndex (LocalVariables|GetL_PathPoint))))) 3e+01)) (* (Math|Vector|GetForwardVector (Math|Rotator|FindLookatRotation _returnvalue (Utilities|Array|Get(acopy) (LocalVariables|GetL_PathPoint) (Utilities|Array|LastIndex (LocalVariables|GetL_PathPoint))))) -1e+01)))) (+ (.Z (Math|Vector|BreakVector (+ (+ _returnvalue (* (Math|Vector|GetRightVector (Math|Rotator|FindLookatRotation _returnvalue (Utilities|Array|Get(acopy) (LocalVariables|GetL_PathPoint) (Utilities|Array|LastIndex (LocalVariables|GetL_PathPoint))))) 3e+01)) (* (Math|Vector|GetForwardVector (Math|Rotator|FindLookatRotation _returnvalue (Utilities|Array|Get(acopy) (LocalVariables|GetL_PathPoint) (Utilities|Array|LastIndex (LocalVariables|GetL_PathPoint))))) -1e+01)))) (Variables|TrackSettings|GetInitPointHeightTrack)))))
  (LocalVariables|SetL_DestinationPoint (select (> (Math|Vector|VectorLength (- (LocalVariables|GetL_BeginPoint) _currentcursorlocation)) (Variables|TrackSettings|GetThrowGrenadeRange)) (+ (LocalVariables|GetL_BeginPoint) (* (Math|Vector|GetForwardVector (Math|Rotator|FindLookatRotation (LocalVariables|GetL_BeginPoint) _currentcursorlocation)) (Variables|TrackSettings|GetThrowGrenadeRange))) (Utilities|Array|Get(acopy) (LocalVariables|GetL_PathPoint) (Utilities|Array|LastIndex (LocalVariables|GetL_PathPoint)))))
  (bind _returnvalue_2 (Game|SpawnActorfromClass "/Game/ATBS/Blueprints/PlayerNPCs/Blueprints/SupportActors/BP_SplineActor.BP_SplineActor_C" (Math|Transform|MakeTransform (LocalVariables|GetL_BeginPoint) (Math|Rotator|FindLookatRotation (LocalVariables|GetL_BeginPoint) (LocalVariables|GetL_DestinationPoint)) "1,1,1") "AlwaysSpawn" 0 0))
  (bind _output_get (Variables|Hide|SetSplineActor _returnvalue_2))
  (bind _output_get_2 (Variables|Hide|SetSpline (Variables|/Game/ATBS/Blueprints/PlayerNPCs/Blueprints/SupportActors/BP_SplineActor.BP_SplineActor_C|GetSpline _output_get)))
  (bind _output_get_3 (LocalVariables|SetL_Spline _output_get_2))
  (Spline|ClearSplinePoints _output_get_3 false)
  (bind _outlaunchvelocity (Game|SuggestProjectileVelocityCustomArc (LocalVariables|GetL_BeginPoint) (LocalVariables|GetL_DestinationPoint) 0.0 (LocalVariables|GetL_ArcParam) :!label _label))
  (bind _outpathpositions (Class|GameplayStatics|BlueprintPredictProjectilePathbyObjectType (LocalVariables|GetL_BeginPoint) _outlaunchvelocity true 2e+01 (Utilities|Array|MakeArray "ObjectTypeQuery1" "ObjectTypeQuery2" "ObjectTypeQuery3") false (Utilities|Array|MakeArray (Variables|PrivateVariable|GetOwnerCharacter)) "None" 2.0 15.0 4.0 0.0))
  (LocalVariables|SetArrayProjectilePath _outpathpositions)
  (for _array_element (LocalVariables|GetArrayProjectilePath)
    (Spline|AddSplinePoint (LocalVariables|GetL_Spline) _array_element "World" true))
  (if (and (< (Spline|GetSplineLength (LocalVariables|GetL_Spline)) (Math|Vector|VectorLength (- (LocalVariables|GetL_BeginPoint) (LocalVariables|GetL_DestinationPoint)))) (not (<= (LocalVariables|GetL_ArcParam) 0.2)))
    (Spline|ClearSplinePoints (LocalVariables|GetL_Spline) true)
    (LocalVariables|SetL_ArcParam (- (LocalVariables|GetL_ArcParam) 0.01))
    (goto _label)
    (else
      (LocalVariables|SetL_DestinationPoint (Utilities|Array|Get(acopy) (LocalVariables|GetArrayProjectilePath) (Utilities|Array|LastIndex (LocalVariables|GetArrayProjectilePath))))
      (return (LocalVariables|GetL_DestinationPoint) (LocalVariables|GetL_BeginPoint) (LocalVariables|GetL_ArcParam)))))

(fn EndDestination
  (params (Location :type Vector))
  (bind _d_endmaterial (Variables|Hide|GetD_EndMaterial))
  (bind _grenaderadiuscolor (Variables|TrackSettings|GetGrenadeRadiusColor))
  (bind _newstaticmeshgrenaderadius (Variables|TrackSettings|GetNewStaticMeshGrenadeRadius))
  (LocalVariables|SetL_Location Location)
  (Rendering|Material|SetVectorParameterValue _d_endmaterial "GridColor" _grenaderadiuscolor :!class /Script/Engine.MaterialInstanceDynamic)
  (Rendering|Material|SetVectorParameterValue _d_endmaterial "LineRadiusColor" _grenaderadiuscolor :!class /Script/Engine.MaterialInstanceDynamic)
  (Rendering|Material|SetVectorParameterValue (Variables|Hide|GetD_FloorMaterial) "Color" (Variables|TrackSettings|GetGrenadeFloorRadiusColor) :!class /Script/Engine.MaterialInstanceDynamic)
  (bind _endpointdestination (Variables|Hide|GetEndPointDestination)
    (:then
      (Transformation|SetActorLocation _endpointdestination (LocalVariables|GetL_Location) false false))
    (:else
      (bind _returnvalue (Game|SpawnActorfromClass "/Game/ATBS/Blueprints/PlayerNPCs/Blueprints/SupportActors/BP_Single_GrenadeRadus.BP_Single_GrenadeRadus_C" (Math|Transform|MakeTransform (LocalVariables|GetL_Location) "0, 0, 0" (Math|Conversions|ToVector(Float) (* (/ (Variables|TrackSettings|GetGrenadeDamageRadius) 1e+02) 2.0))) "Undefined" 0 (Variables|Hide|GetD_EndMaterial) (Variables|Hide|GetD_FloorMaterial) 0 (select (Utilities|IsValid _newstaticmeshgrenaderadius) _newstaticmeshgrenaderadius 0)))
      (Variables|Hide|SetEndPointDestination _returnvalue)))
  (Variables|Hide|SetLastCursorPosition (LocalVariables|GetL_Location)))

(fn ClearPath
  (bind _massivesphere (Variables|Hide|GetMassiveSphere))
  (bind _splineactor (Variables|Hide|GetSplineActor)
    (:then
      (Actor|DestroyActor _splineactor))
    (:else
      _))
  (Utilities|Array|Clear (Variables|Hide|GetOldsMeshesPath))
  (if (> (Utilities|Array|Length (Variables|Hide|GetMassiveSphere)) 0)
    (for _array_element _massivesphere
      (Actor|DestroyActor _array_element))
    (Utilities|Array|Clear _massivesphere)
    (Variables|PrivateVariable|SetTrackWasCreated false)
    (return)
    (else
      (Variables|PrivateVariable|SetTrackWasCreated false)
      (return))))

(fn AddStaticMesh
  (bind (_spline _returnvalue) (CallFunction|GetSplineLenght))
  (bind _spline_2 (Variables|Hide|GetSpline))
  (bind _scalepath (Variables|TrackSettings|GetScalePath))
  (bind _returnvalue_2 (Math|Vector2D|MakeVector2D _scalepath _scalepath))
  (Rendering|Material|SetVectorParameterValue (Variables|Hide|GetD_Material) "Color" (Variables|TrackSettings|GetTrackColor) :!class /Script/Engine.MaterialInstanceDynamic)
  (LocalVariables|SetL_Spline _spline)
  (for _index (range 0 _returnvalue)
    (LocalVariables|SetL_SplineIndex _index)
    (bind _smc (Default|CreateSplineMesh (Variables|Hide|GetSplineActor) (Variables|Hide|GetD_Material) (LocalVariables|GetL_SplineIndex) _returnvalue (LocalVariables|GetL_Spline) "NewEnumerator2"))
    (bind _output_get (LocalVariables|SetL_SMC _smc))
    (Utilities|Array|Add (Variables|Hide|GetOldsMeshesPath) _output_get)
    (SplineMesh|SetEndScale (LocalVariables|GetL_SMC) _returnvalue_2 false :!class /Script/Engine.SplineMeshComponent)
    (SplineMesh|SetStartScale (LocalVariables|GetL_SMC) _returnvalue_2 false :!class /Script/Engine.SplineMeshComponent)
    (SplineMesh|SetStartandEnd (LocalVariables|GetL_SMC) (.Location (Spline|GetLocationandTangentatSplinePoint (LocalVariables|GetL_Spline) (LocalVariables|GetL_SplineIndex) "World")) (.Tangent (Spline|GetLocationandTangentatSplinePoint (LocalVariables|GetL_Spline) (LocalVariables|GetL_SplineIndex) "World")) (.Location (Spline|GetLocationandTangentatSplinePoint (LocalVariables|GetL_Spline) (+ (LocalVariables|GetL_SplineIndex) 1) "World")) (Math|Vector|ClampVectorSize (.Tangent (Spline|GetLocationandTangentatSplinePoint (LocalVariables|GetL_Spline) (+ (LocalVariables|GetL_SplineIndex) 1) "World")) 0.0 5e+01) true :!class /Script/Engine.SplineMeshComponent)
    (if (== (LocalVariables|GetL_SplineIndex) 0)
      (CallFunction|AddSphereMeshatLinePath (.Location (Spline|GetLocationandTangentatSplinePoint (LocalVariables|GetL_Spline) (LocalVariables|GetL_SplineIndex) "World")))))
  (CallFunction|AddSphereMeshatLinePath (Spline|GetLocationatSplinePoint _spline_2 (Spline|GetNumberOfSplinePoints _spline_2) "World"))
  (return (LocalVariables|GetL_SMC)))

(fn GetSplineLenght
  (bind _spline (Variables|Hide|GetSpline))
  (return _spline (- (Spline|GetNumberOfSplinePoints _spline) 2)))

(fn UpdateCurrentSpline
  (LocalVariables|SetL_Spline (Variables|/Game/ATBS/Blueprints/PlayerNPCs/Blueprints/SupportActors/BP_SplineActor.BP_SplineActor_C|GetSpline (Variables|Hide|GetSplineActor)))
  (Spline|UpdateSpline (LocalVariables|GetL_Spline))
  (return))

(fn AddSphereMeshatLinePath
  (params (Location :type Vector))
  (bind _returnvalue (Game|SpawnActorfromClass "/Game/ATBS/Blueprints/PlayerNPCs/Blueprints/SupportActors/BP_Sphere_SM.BP_Sphere_SM_C" (Math|Transform|MakeTransform Location "0.000000,0.000000, 0" "0.100000,0.100000,0.100000") "Undefined" 0 (Variables|Hide|GetD_Material) 0))
  (Utilities|Array|Add (Variables|Hide|GetMassiveSphere) _returnvalue))

(fn SwitchMovement
  (params (Selection :type E_SelectorForUse%20Enum))
  (bind _returnvalue (Game|GetPlayerController 0))
  (bind _hitresult (Game|Player|GetHitResultUnderCursorbyChannel _returnvalue "TraceTypeQuery2" true))
  (bind (_bblockinghit _binitialoverlap _time _location _impactpoint _normal _impactnormal _physmat _hitactor _hitcomponent _hitbonename _hititem) (Collision|BreakHitResult _hitresult))
  (switch Utilities|FlowControl|Switch|SwitchonE_SelectorForUse Selection
    (:NewEnumerator1
      (return _location))
    (:NewEnumerator2
      (bind _asbp_experemental_hex_grid (Utilities|Casting|CastToBP_Experemental_HexGrid _hitactor))
      (return (Utilities|Array|Get(acopy) (Variables|/Game/ATBS/ExperementalGrid/Blueprints/BP_Experemental_HexGrid.BP_Experemental_HexGrid_C|GetArrayHexGridLocation _asbp_experemental_hex_grid) _hititem)))))