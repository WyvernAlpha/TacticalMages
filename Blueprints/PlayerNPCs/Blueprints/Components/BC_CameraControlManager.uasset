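; Actor component that handles movement and orbit camera controls for its owner's instigator pawn.
; On BeginPlay it caches that pawn and its spring arm and turns on camera rotation lag.
; Axis events move the pawn relative to control yaw unless the camera is focused, and zoom by clamping arm length with optional inversion.
; While right mouse is held, yaw drives controller rotation and pitch rotates the spring arm within limits.
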(event Custom|MoveForward
  (params (AxisValue :type Float%20%28single-precision%29))
  (if (not (Variables|Hide|GetCameraWasFocused?))
    (Pawn|Input|AddMovementInput (Variables|Default|GetGetInstigatorOwner) (Math|Vector|GetForwardVector (Math|Rotator|MakeRotator 0.0 0.0 (.Yaw (Math|Rotator|BreakRotator (Pawn|GetControlRotation (Variables|Default|GetGetInstigatorOwner) :!class /Script/Engine.Pawn))))) AxisValue false)))

(event Custom|MoveRight
  (params (AxisValue :type Float%20%28single-precision%29))
  (if (not (Variables|Hide|GetCameraWasFocused?))
    (Pawn|Input|AddMovementInput (Variables|Default|GetGetInstigatorOwner) (Math|Vector|GetRightVector (Math|Rotator|MakeRotator 0.0 0.0 (.Yaw (Math|Rotator|BreakRotator (Pawn|GetControlRotation (Variables|Default|GetGetInstigatorOwner) :!class /Script/Engine.Pawn))))) AxisValue false)))

(event Custom|CameraRotatePitch
  (params (AxisValue :type Float%20%28single-precision%29))
  (if (Variables|Default|GetHoldRightMouseButton)
    (Transformation|SetRelativeRotation (Variables|Default|GetSpringArm) (Math|Rotator|MakeRotator 0.0 (Math|Float|ClampAngle (+ (* AxisValue (Variables|Default|GetCameraRotationSpeed)) (.pitch (Variables|/Script/Engine.SceneComponent|GetRelativeRotation (Variables|Default|GetSpringArm)))) -9e+01 (Variables|Default|GetMaxAnglePitch)) 0.0) false false)))

(event Custom|CameraZoom
  (params (AxisValue :type Float%20%28single-precision%29))
  (Variables|/Script/Engine.SpringArmComponent|SetTargetArmLength (Variables|Default|GetSpringArm) (Math|Float|Clamp(Float) (+ (Variables|/Script/Engine.SpringArmComponent|GetTargetArmLength (Variables|Default|GetSpringArm)) (* AxisValue (* (Variables|Default|GetCameraZoomingSpeed) (Math|Float|SelectFloat 5e+01 -5e+01 (Variables|Default|GetReverseForCameraZoom))))) (Variables|Default|GetZoomInMin) (Variables|Default|GetZoomOutMax))))

(event Custom|CameraRotateYaw
  (params (AxisValue :type Float%20%28single-precision%29))
  (if (Variables|Default|GetHoldRightMouseButton)
    (Pawn|Input|AddControllerYawInput (Variables|Default|GetGetInstigatorOwner) (* AxisValue (Variables|Default|GetCameraRotationSpeed)))))

(event EventBeginPlay
  (bind _returnvalue (Components|GetOwner))
  (bind _instigator (Variables|/Script/Engine.Actor|GetInstigator _returnvalue))
  (Variables|Default|SetGetInstigatorOwner _instigator)
  (bind _output_get (Variables|Default|SetSpringArm (Actor|GetComponentbyClass _instigator "/Script/Engine.SpringArmComponent")))
  (Variables|/Script/Engine.SpringArmComponent|SetbEnableCameraRotationLag _output_get true)
  (Variables|/Script/Engine.SpringArmComponent|SetCameraRotationLagSpeed (Variables|Default|GetSpringArm) 2e+01))

(event EventTick
  (params (DeltaSeconds :type Float%20%28single-precision%29)))