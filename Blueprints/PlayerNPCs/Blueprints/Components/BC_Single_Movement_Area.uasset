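; Actor component for a character that displays its movement range by spawning a BP_SphereArea around it.
; It reads path lengths from the sibling BC_Single_DrawPath component to scale the area and an inner radius, which is clamped to the capsule diameter or hidden.
; Each draw destroys the previous area and spawns the new one at the owner's grid-snapped position, raised in Z.
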(event Custom|Event_DrawArea
  (if (not (Variables|Debug|GetHideArea?))
    (CallFunction|SpawnAreaMovement)))

(event Custom|DestroyZone
  (bind _spherearea (Variables|Default|GetSphereArea)
    (:then
      (Actor|DestroyActor _spherearea))
    (:else)))

(event Custom|ResetMovementArea
  (Variables|Default|SetRadiusZoneMovement (Variables|/Game/ATBS/Blueprints/PlayerNPCs/Blueprints/Components/BC_Single_DrawPath.BC_Single_DrawPath_C|GetMaxPathLenght (Variables|Default|GetPathMovementComponent)))
  (CallFunction|DestroyZone))

(event EventBeginPlay
  (bind _returnvalue (Components|GetOwner))
  (Variables|Default|SetControllerOwner (AI|GetAIController _returnvalue))
  (bind _ascharacter (Utilities|Casting|CastToCharacter _returnvalue))
  (bind _output_get (Variables|Default|SetOwnerComponent _ascharacter))
  (Utilities|IsValid (Actor|GetComponentbyClass _output_get "/Game/ATBS/Blueprints/PlayerNPCs/Blueprints/Components/BC_Single_DrawPath.BC_Single_DrawPath_C")
    (:Is%20Valid
      (bind _output_get_2 (Variables|Default|SetPathMovementComponent (Actor|GetComponentbyClass _output_get "/Game/ATBS/Blueprints/PlayerNPCs/Blueprints/Components/BC_Single_DrawPath.BC_Single_DrawPath_C")))
      (Variables|Default|SetRadiusZoneMovement (Variables|/Game/ATBS/Blueprints/PlayerNPCs/Blueprints/Components/BC_Single_DrawPath.BC_Single_DrawPath_C|GetMaxPathLenght _output_get_2)))))

(fn SpawnAreaMovement
  (bind _capsuleradius (CallFunction|SetPlayerRadius))
  (bind _pathmovementcomponent (Variables|Default|GetPathMovementComponent))
  (bind _pathmovementcomponent_2 (Variables|Default|GetPathMovementComponent))
  (bind _currentpathlenght (Variables|/Game/ATBS/Blueprints/PlayerNPCs/Blueprints/Components/BC_Single_DrawPath.BC_Single_DrawPath_C|GetCurrentPathLenght _pathmovementcomponent))
  (bind _longdistance (Variables|/Game/ATBS/Blueprints/PlayerNPCs/Blueprints/Components/BC_Single_DrawPath.BC_Single_DrawPath_C|GetLongDistance _pathmovementcomponent_2))
  (bind _currentpathlenght_2 (Variables|/Game/ATBS/Blueprints/PlayerNPCs/Blueprints/Components/BC_Single_DrawPath.BC_Single_DrawPath_C|GetCurrentPathLenght _pathmovementcomponent_2))
  (bind _returnvalue (- _currentpathlenght_2 _longdistance))
  (bind _returnvalue_2 (/ _currentpathlenght 1e+02))
  (bind _returnvalue_3 (Math|Conversions|ToVector(Float) _returnvalue_2))
  (bind _returnvalue_4 (* _returnvalue 2.0))
  (bind (_x _y) (Math|Vector|BreakVector _returnvalue_3))
  (bind _returnvalue_5 (Math|Float|Max(Float) _returnvalue_4 _capsuleradius))
  (bind _returnvalue_6 (/ _returnvalue_5 1e+02))
  (CallFunction|ResetMovementArea)
  (bind _output_get (Variables|Default|SetOwnerPosition (CallFunction|SnaptoGridLogic)))
  (bind _returnvalue_7 (Game|SpawnActorfromClass "/Game/ATBS/Blueprints/PlayerNPCs/Blueprints/SupportActors/BP_SphereArea.BP_SphereArea_C" (Math|Transform|MakeTransform (+ _output_get "0, 0,200.000000") "0, 0, 0" (Math|Vector|MakeVector _x _y 15.0)) "AlwaysSpawn" 0 0))
  (Variables|Default|SetSphereArea _returnvalue_7)
  (if (<= (Variables|/Game/ATBS/Blueprints/PlayerNPCs/Blueprints/Components/BC_Single_DrawPath.BC_Single_DrawPath_C|GetCloseDistance (Variables|Default|GetPathMovementComponent)) (CallFunction|SetPlayerRadius))
    (Development|SetHiddeninGame (Variables|/Game/ATBS/Blueprints/PlayerNPCs/Blueprints/SupportActors/BP_SphereArea.BP_SphereArea_C|GetFirstRadius (Variables|Default|GetSphereArea)) true false)
    (else
      (Transformation|SetWorldScale3D (Variables|/Game/ATBS/Blueprints/PlayerNPCs/Blueprints/SupportActors/BP_SphereArea.BP_SphereArea_C|GetFirstRadius (Variables|Default|GetSphereArea)) (Math|Vector|MakeVector _returnvalue_6 _returnvalue_6 (.z (Transformation|GetWorldScale (Variables|/Game/ATBS/Blueprints/PlayerNPCs/Blueprints/SupportActors/BP_SphereArea.BP_SphereArea_C|GetFirstRadius (Variables|Default|GetSphereArea)))))))))

(fn SnaptoGridLogic
  (bind _calculationaccuracy (Variables|Default|GetCalculationAccuracy))
  (bind _ownercomponent (Variables|Default|GetOwnerComponent))
  (bind _returnvalue (Transformation|GetActorLocation _ownercomponent))
  (return (Math|Vector|MakeVector (Math|Float|SnapToGrid(Float) (.x _returnvalue) _calculationaccuracy) (Math|Float|SnapToGrid(Float) (.y _returnvalue) _calculationaccuracy) (.z _returnvalue))))

(fn SetPlayerRadius
  (return (* (Variables|/Script/Engine.CapsuleComponent|GetCapsuleRadius (Variables|/Script/Engine.Character|GetCapsuleComponent (Variables|Default|GetOwnerComponent))) 2.0)))