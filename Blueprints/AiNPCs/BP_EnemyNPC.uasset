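; Enemy NPC character that repeatedly relocates between cover points and ragdolls when its health runs out.
; AiMoveAgain stands it up and queries the cover-finder component, whose results are chosen by health and player visibility.
; It moves to a random unoccupied pick, or a random reachable point without cover, crouches in cover and fires AiMovingFinish.
; It affects dynamic navmesh generation while stationary, switching this off to move.
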(event DArrayCoverPosition(BC_FindCoverPoints)
  (params (WasFoundAndCanBeUsed :type Boolean) (ArrayCoverLocation :type Array%20of%20Vectors) (PlayerCanSeeEnemy :type Array%20of%20Vectors) (PlayerSeeNPC? :type Boolean) (ShootingLocation :type Array%20of%20Vectors) (IsCanShooting? :type Boolean) (ArrayLocationPlayerNOTSeeNPCs :type Array%20of%20Vectors) (PlayerNOTSeeNPCs? :type Boolean))
  (Variables|Default|SetCanCover WasFoundAndCanBeUsed)
  (if (Variables|Default|GetCanCover)
    (Variables|Default|SetArrayCoverPoints (select (and (< (Variables|Default|GetHealth) 55.0) PlayerNOTSeeNPCs?) ArrayLocationPlayerNOTSeeNPCs (select (and IsCanShooting? (> (Variables|Default|GetHealth) 55.0)) ShootingLocation (select PlayerSeeNPC? PlayerCanSeeEnemy ArrayCoverLocation))))
    (CallFunction|EventAIMovetoPointDestination)
    (else
      (CallFunction|EventAIMovetoPointDestination))))

(event Custom|Death
  (bind _mesh (Variables|Character|GetMesh))
  (Utilities|FlowControl|DoOnce false
    (:Completed
      (Class|Pawn|SetCanAffectNavigationGeneration false)
      (Collision|SetCollisionEnabled (Variables|Collision|GetCapsuleComponent) "NoCollision")
      (Physics|SetSimulatePhysics _mesh true)
      (Collision|SetCollisionEnabled _mesh "PhysicsOnly")
      (Pawn|Components|CharacterMovement|SetMovementMode (Variables|Character|GetCharacterMovement) "MOVE_None" 0)
      (Variables|Default|SetIsDead? true))))

(event Custom|AiMoveAgain
  (Class|Pawn|SetCanAffectNavigationGeneration false) ; If alive, Disable Collision for correct movement on the nav mesh
  (if (Variables|Default|GetCanCover)
    (Character|UnCrouch)
    (elif (Variables|Default|GetIsDead?) ; Check if Dead
      (Default|CallAiMovingFinish) ; Calls Dispatcher
      (else
        (Default|EventFindCoverPoints (Variables|Default|GetBC_FindCoverPoints) self 0.0)))))

(event Custom|Event_AI_MoveToPointDestination
  (bind _arraycoverpoints (Variables|Default|GetArrayCoverPoints))
  (Utilities|FlowControl|Delay 0.2) ; Wait
  (Variables|Default|SetPointDestination (select (Variables|Default|GetCanCover) (Utilities|Array|Get(acopy) _arraycoverpoints (Math|Random|RandomIntegerinRange 0 (Utilities|Array|LastIndex _arraycoverpoints))) (.RandomLocation (AI|Navigation|GetRandomReachablePointinRadius (Transformation|GetActorLocation) 1e+03))) :!label _label) ; Set Point
  (bind _returnvalue (Collision|SphereOverlapActors (Variables|Default|GetPointDestination) 5e+01 (Utilities|Array|MakeArray "ObjectTypeQuery3") 0 (Utilities|Array|MakeArray self))) ; Check - Has a pawn in current position
  (if _returnvalue
    (goto _label)
    (else
      (AI|AIMoveTo self (Variables|Default|GetPointDestination) 0 5.0 false ; If no found Pawn in current position - can Movement
        (:OnSuccess
          (if (Variables|Default|GetCanCover)
            (Character|Crouch)
            (Utilities|FlowControl|Delay 1.0)))
        (:OnFail
          _))
      (Default|CallAiMovingFinish) ; If Finish movement - calls Dispatcher
      (if (not (Variables|Default|GetIsDead?)) ; If Alive (Because can be Dead in moment movement)
        (Class|Pawn|SetCanAffectNavigationGeneration true) ; And resturn collision setting
      ))))

(event Game|Damage|EventAnyDamage
  (params (Damage :type Float%20%28single-precision%29) (DamageType :type Damage%20Type%20Object%20Reference) (InstigatedBy :type Controller%20Object%20Reference) (DamageCauser :type Actor%20Object%20Reference))
  (bind _output_get (Variables|Default|SetHealth (Math|Float|Clamp(Float) (- (Variables|Default|GetHealth) Damage) 0.0 1e+02))) ; Set Heath
  (if (<= _output_get 0.0) ; If Health <= 0 - Death
    (CallFunction|Death)))

(event EventOnStartCrouch
  (params (HalfHeightAdjust :type Float%20%28single-precision%29) (ScaledHalfHeightAdjust :type Float%20%28single-precision%29)))

(event EventBeginPlay
  (Class|Pawn|SetCanAffectNavigationGeneration true) ; Enable Nav Detect for Dynamic Nav Mesh
)

(event EventOnEndCrouch
  (params (HalfHeightAdjust :type Float%20%28single-precision%29) (ScaledHalfHeightAdjust :type Float%20%28single-precision%29))
  (if (Variables|Default|GetIsDead?) ; Check if Dead
    (Default|CallAiMovingFinish) ; Calls Dispatcher
    (else
      (Default|EventFindCoverPoints (Variables|Default|GetBC_FindCoverPoints) self 0.0))))

(fn ConstructionScript)