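; Experimental grid actor that builds a box, offset-box or hex tile grid in its construction script.
; CreateGrid dispatches on GridOption, placing tiles as instances of one instanced static mesh and recording their locations, with optional X/Y text labels.
; In navmesh mode, vertical sphere traces snap tiles to surfaces, keeping only points that are on the navmesh, path-reachable from the actor and clear of WorldStatic objects.
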(event EventBeginPlay)

(event Collision|EventActorBeginOverlap
  (params (OtherActor :type Actor%20Object%20Reference)))

(fn ConstructionScript
  (bind _returnvalue (AddComponent|AddInstancedStaticMeshComponent false))
  (bind _output_get (Variables|Default|SetMasterInstance _returnvalue))
  (Components|StaticMesh|SetStaticMesh _output_get (Utilities|Select :Index (Variables|Default|GetGridOption) :NewEnumerator3 0 :NewEnumerator0 "/Engine/VREditor/BasicMeshes/SM_Cube_02.SM_Cube_02" :NewEnumerator2 "/Engine/VREditor/BasicMeshes/SM_Cube_02.SM_Cube_02" :NewEnumerator1 "/Game/ATBS/ExperementalGrid/StaticMeshes/SM_HexTile.SM_HexTile"))
  (Utilities|Array|Clear (Variables|Default|GetArrayHexGridLocation))
  (CallFunction|CreateGrid))

(fn ExperementalBoxGrid
  (params (X :type Integer) (Y :type Integer) (Sector%20Size :type Float%20%28single-precision%29))
  (bind _scale (Variables|Default|GetScale))
  (bind _returnvalue (Math|Vector|MakeVector _scale _scale 0.1))
  (LocalVariables|SetL_SelectIndex (< (Variables|Default|GetScale) 1.0))
  (LocalVariables|SetL_InitLocation (- (Transformation|GetActorLocation) (Variables|/Script/Engine.SceneComponent|GetRelativeLocation (Variables|Default|GetDefaultSceneRoot))))
  (bind (_current_point _total_points _0_1_phase _poly_center _x_row _y_row) (Utilities|2DGridExecutionMacro (select (LocalVariables|GetL_SelectIndex) (/ Sector%20Size (select (LocalVariables|GetL_SelectIndex) (/ 1.0 (Variables|Default|GetScale)) Sector%20Size)) (* Sector%20Size (Variables|Default|GetScale))) (LocalVariables|GetL_InitLocation) X Y)
    (:Per%20Poly%20Execution
      (Variables|Default|SetCurrentGrid_X _x_row)
      (Variables|Default|SetCurrentGrid_Y _y_row)
      (LocalVariables|SetL_Location _poly_center)
      (if (Variables|Default|GetCalculateNavMesh?)
        (CallFunction|CalculateGridtoNavMesh (LocalVariables|GetL_Location) _returnvalue)
        (else
          (bind _returnvalue_2 (Components|InstancedStaticMesh|AddInstance (Variables|Default|GetMasterInstance) (Math|Transform|MakeTransform (LocalVariables|GetL_Location) "0, 0, 0" _returnvalue)))
          (bind _returnvalue_3 (Utilities|Array|Add (Variables|Default|GetArrayHexGridLocation) (.location (.OutInstanceTransform (Components|InstancedStaticMesh|GetInstanceTransform (Variables|Default|GetMasterInstance) _returnvalue_2 true)))))
          (if (Variables|Default|GetShowNumeration?)
            (CallFunction|AddNumerationText (Utilities|Array|Get(acopy) (Variables|Default|GetArrayHexGridLocation) _returnvalue_3))))))))

(fn ExperementalHexGrid
  (params (MaxGrid_X :type Integer) (MaxGrid_Y :type Integer) (ScaleHex :type Float%20%28single-precision%29))
  (bind _spacing_x (Variables|Default|GetSpacing_X))
  (bind _spacing_y (Variables|Default|GetSpacing_Y))
  (bind _returnvalue (Math|Vector|MakeVector ScaleHex ScaleHex 1.0))
  (LocalVariables|SetL_SelectIndex (< ScaleHex 1.0))
  (for _index (range 0 MaxGrid_X)
    (Variables|Default|SetCurrentGrid_X _index)
    (for _index_2 (range 0 MaxGrid_Y)
      (Variables|Default|SetCurrentGrid_Y _index_2)
      (LocalVariables|SetL_Location (+ (Math|Vector|MakeVector (* (* (/ (* MaxGrid_X (Variables|Default|GetSpacing_X)) 2.0) ScaleHex) -1.0) (* (* (/ (* MaxGrid_Y (Variables|Default|GetSpacing_Y)) 2.0) ScaleHex) -1.0) 0.0) (select (== (Math|Integer|%(Integer) (Variables|Default|GetCurrentGrid_X) 2) 0) (Math|Vector|MakeVector (* (Variables|Default|GetCurrentGrid_X) (select (LocalVariables|GetL_SelectIndex) (/ _spacing_x (select (LocalVariables|GetL_SelectIndex) (/ 1.0 ScaleHex) ScaleHex)) (* _spacing_x ScaleHex))) (+ (* (Variables|Default|GetCurrentGrid_Y) (select (LocalVariables|GetL_SelectIndex) (/ _spacing_y (select (LocalVariables|GetL_SelectIndex) (/ 1.0 ScaleHex) ScaleHex)) (* _spacing_y ScaleHex))) (/ (select (LocalVariables|GetL_SelectIndex) (/ _spacing_y (select (LocalVariables|GetL_SelectIndex) (/ 1.0 ScaleHex) ScaleHex)) (* _spacing_y ScaleHex)) 2.0)) 0.0) (Math|Vector|MakeVector (* (Variables|Default|GetCurrentGrid_X) (select (LocalVariables|GetL_SelectIndex) (/ _spacing_x (select (LocalVariables|GetL_SelectIndex) (/ 1.0 ScaleHex) ScaleHex)) (* _spacing_x ScaleHex))) (* (Variables|Default|GetCurrentGrid_Y) (select (LocalVariables|GetL_SelectIndex) (/ _spacing_y (select (LocalVariables|GetL_SelectIndex) (/ 1.0 ScaleHex) ScaleHex)) (* _spacing_y ScaleHex))) 0.0))))
      (if (Variables|Default|GetCalculateNavMesh?)
        (CallFunction|CalculateGridtoNavMesh (LocalVariables|GetL_Location) _returnvalue)
        (else
          (bind _returnvalue_2 (Components|InstancedStaticMesh|AddInstance (Variables|Default|GetMasterInstance) (Math|Transform|MakeTransform (LocalVariables|GetL_Location) "0, 0, 0" _returnvalue)))
          (bind _returnvalue_3 (Utilities|Array|Add (Variables|Default|GetArrayHexGridLocation) (.location (.OutInstanceTransform (Components|InstancedStaticMesh|GetInstanceTransform (Variables|Default|GetMasterInstance) _returnvalue_2 true)))))
          (if (Variables|Default|GetShowNumeration?)
            (CallFunction|AddNumerationText (Utilities|Array|Get(acopy) (Variables|Default|GetArrayHexGridLocation) _returnvalue_3))))))))

(fn ExperementalBoxGridOffset
  (params (Sector%20Size :type Float%20%28single-precision%29))
  (bind _scale (Variables|Default|GetScale))
  (bind _returnvalue (Math|Vector|MakeVector _scale _scale 0.1))
  (LocalVariables|SetL_SelectIndex (< (Variables|Default|GetScale) 1.0))
  (LocalVariables|SetL_InitLocation (- (Transformation|GetActorLocation) (Variables|/Script/Engine.SceneComponent|GetRelativeLocation (Variables|Default|GetDefaultSceneRoot))))
  (LocalVariables|SetLSectorSize (select (LocalVariables|GetL_SelectIndex) (/ Sector%20Size (select (LocalVariables|GetL_SelectIndex) (/ 1.0 (Variables|Default|GetScale)) Sector%20Size)) (* Sector%20Size (Variables|Default|GetScale))))
  (bind (_current_point _total_points _0_1_phase _poly_center _x_row _y_row) (Utilities|2DGridExecutionMacro (LocalVariables|GetLSectorSize) (LocalVariables|GetL_InitLocation) (Variables|Default|GetMaxGrid_X) (Variables|Default|GetMaxGrid_Y))
    (:Per%20Poly%20Execution
      (Variables|Default|SetCurrentGrid_X _x_row)
      (Variables|Default|SetCurrentGrid_Y _y_row)
      (LocalVariables|SetL_Location (Math|Vector|MakeVector (.X (Math|Vector|BreakVector _poly_center)) (- (select (== (Math|Integer|%(Integer) (Variables|Default|GetCurrentGrid_X) 2) 0) (+ (* (Variables|Default|GetCurrentGrid_Y) (LocalVariables|GetLSectorSize)) (/ (LocalVariables|GetLSectorSize) 2.0)) (* (Variables|Default|GetCurrentGrid_Y) (LocalVariables|GetLSectorSize))) (/ (* (Variables|Default|GetMaxGrid_Y) (LocalVariables|GetLSectorSize)) 2.0)) (.Z (Math|Vector|BreakVector _poly_center))))
      (if (Variables|Default|GetCalculateNavMesh?)
        (CallFunction|CalculateGridtoNavMesh (LocalVariables|GetL_Location) _returnvalue)
        (else
          (bind _returnvalue_2 (Components|InstancedStaticMesh|AddInstance (Variables|Default|GetMasterInstance) (Math|Transform|MakeTransform (LocalVariables|GetL_Location) "0, 0, 0" _returnvalue)))
          (bind _returnvalue_3 (Utilities|Array|Add (Variables|Default|GetArrayHexGridLocation) (.location (.OutInstanceTransform (Components|InstancedStaticMesh|GetInstanceTransform (Variables|Default|GetMasterInstance) _returnvalue_2 true)))))
          (if (Variables|Default|GetShowNumeration?)
            (CallFunction|AddNumerationText (Utilities|Array|Get(acopy) (Variables|Default|GetArrayHexGridLocation) _returnvalue_3))))))))

(fn ExperementalHexGridCyrcle
  (params (MaxGrid_X :type Integer) (MaxGrid_Y :type Integer) (ScaleHex :type Float%20%28single-precision%29))
  (bind _spacing_y (Variables|Default|GetSpacing_Y))
  (LocalVariables|SetL_SelectIndex (< ScaleHex 1.0))
  (for _index (range 0 MaxGrid_X)
    (Variables|Default|SetCurrentGrid_X _index)
    (for _index_2 (range 0 MaxGrid_Y)
      (Variables|Default|SetCurrentGrid_Y _index_2)
      (Utilities|FlowControl|Sequence
        (:then_0
          (bind _returnvalue (AddComponent|AddTextRenderComponent false (Math|Transform|MakeTransform (Math|Vector|MakeVector (.X (Math|Vector|BreakVector (select (== (Math|Integer|%(Integer) (Variables|Default|GetCurrentGrid_X) 2) 0) (Math|Vector|MakeVector (+ (* (Variables|Default|GetCurrentGrid_Y) _spacing_y) (/ _spacing_y 2.0)) (* (Variables|Default|GetCurrentGrid_X) (Variables|Default|GetSpacing_X)) 0.0) (Math|Vector|MakeVector (* (Variables|Default|GetCurrentGrid_Y) _spacing_y) (* (Variables|Default|GetCurrentGrid_X) (Variables|Default|GetSpacing_X)) 0.0)))) (.Y (Math|Vector|BreakVector (select (== (Math|Integer|%(Integer) (Variables|Default|GetCurrentGrid_X) 2) 0) (Math|Vector|MakeVector (+ (* (Variables|Default|GetCurrentGrid_Y) _spacing_y) (/ _spacing_y 2.0)) (* (Variables|Default|GetCurrentGrid_X) (Variables|Default|GetSpacing_X)) 0.0) (Math|Vector|MakeVector (* (Variables|Default|GetCurrentGrid_Y) _spacing_y) (* (Variables|Default|GetCurrentGrid_X) (Variables|Default|GetSpacing_X)) 0.0)))) (+ (.Z (Math|Vector|BreakVector (select (== (Math|Integer|%(Integer) (Variables|Default|GetCurrentGrid_X) 2) 0) (Math|Vector|MakeVector (+ (* (Variables|Default|GetCurrentGrid_Y) _spacing_y) (/ _spacing_y 2.0)) (* (Variables|Default|GetCurrentGrid_X) (Variables|Default|GetSpacing_X)) 0.0) (Math|Vector|MakeVector (* (Variables|Default|GetCurrentGrid_Y) _spacing_y) (* (Variables|Default|GetCurrentGrid_X) (Variables|Default|GetSpacing_X)) 0.0)))) 5e+01)) "0,180.000000, 0" "1,1,1.000000")))
          (Rendering|Components|TextRender|SetText _returnvalue (CallFunction|StringGridNumber (Variables|Default|GetCurrentGrid_X) (Variables|Default|GetCurrentGrid_Y))))
        (:then_1
          (AddComponent|AddStaticMeshComponent false (Math|Transform|MakeTransform (select (== (Math|Integer|%(Integer) (Variables|Default|GetCurrentGrid_X) 2) 0) (Math|Vector|MakeVector (+ (* (Variables|Default|GetCurrentGrid_Y) _spacing_y) (/ _spacing_y 2.0)) (* (Variables|Default|GetCurrentGrid_X) (Variables|Default|GetSpacing_X)) 0.0) (Math|Vector|MakeVector (* (Variables|Default|GetCurrentGrid_Y) _spacing_y) (* (Variables|Default|GetCurrentGrid_X) (Variables|Default|GetSpacing_X)) 0.0)) "0,90.000000, 0" (Math|Vector|MakeVector ScaleHex ScaleHex 1.0))))))))

(fn CreateGrid
  (switch Utilities|FlowControl|Switch|SwitchonE_GridOption (Variables|Default|GetGridOption)
    (:NewEnumerator0
      (CallFunction|ExperementalBoxGrid (Variables|Default|GetMaxGrid_X) (Variables|Default|GetMaxGrid_Y) 1e+02))
    (:NewEnumerator2
      (CallFunction|ExperementalBoxGridOffset 1e+02))
    (:NewEnumerator1
      (CallFunction|ExperementalHexGrid (Variables|Default|GetMaxGrid_X) (Variables|Default|GetMaxGrid_Y) (Variables|Default|GetScale)))))

(fn ConvertLocationtoWorldSpace
  (params (Relative :type Vector))
  (return (+ (Transformation|GetActorLocation) Relative)))

(fn StringGridNumber
  (params (For%20X :type Integer) (For%20Y :type Integer))
  (return (Utilities|Text|ToText(String) (Utilities|String|Append "X" (Utilities|String|ToString(Integer) For%20X) " - " "Y" (Utilities|String|ToString(Integer) For%20Y)))))

(fn AddNumerationText
  (params (InVec :type Vector))
  (bind (_x _y _z) (Math|Vector|BreakVector InVec))
  (bind _returnvalue (AddComponent|AddTextRenderComponent true (Math|Transform|MakeTransform (Math|Vector|MakeVector _x _y (+ _z 5e+01)) "0,180.000000, 0" "1,1,1.000000")))
  (Rendering|Components|TextRender|SetText _returnvalue (CallFunction|StringGridNumber (Variables|Default|GetCurrentGrid_X) (Variables|Default|GetCurrentGrid_Y))))

(fn CalculateGridtoNavMesh
  (params (Location :type Vector) (World%20Transform%20Scale :type Vector))
  (bind _world (CallFunction|ConvertLocationtoWorldSpace Location))
  (bind _returnvalue (Transformation|GetActorUpVector))
  (bind _outhits (Collision|MultiSphereTraceByChannel (+ _world (* _returnvalue 5e+02)) (+ _world (* _returnvalue -5e+02)) 1e+01 "TraceTypeQuery4" false 0 "None" true "(R=1.000000,G=0.000000,B=0.000000,A=1.000000)" "(R=0.000000,G=1.000000,B=0.000000,A=1.000000)" 2.0))
  (LocalVariables|SetL_ArrayOutHits _outhits)
  (bind _array_element (Utilities|Array|ForEachLoopwithBreak (LocalVariables|GetL_ArrayOutHits))
    (:LoopBody
      (LocalVariables|SetL_ImpactLocation (.impactpoint _array_element))
      (LocalVariables|SetL_NormalRotation "0, 0, 0")
      (if (not (== (Utilities|GetClass (.hitactor _array_element)) "/Game/ATBS/Blueprints/AiNPCs/BP_EnemyNPC.BP_EnemyNPC_C"))
        (if (not (== (Utilities|GetClass (.hitactor _array_element)) "/Game/ATBS/Blueprints/PlayerNPCs/Blueprints/BP_Single_TestNPC.BP_Single_TestNPC_C"))
          (bind _returnvalue_2 (Class|NavigationSystem|FindPathtoLocationSynchronously (Transformation|GetActorLocation) (LocalVariables|GetL_ImpactLocation)))
          (if (.ReturnValue (AI|Navigation|ProjectPointtoNavigation (LocalVariables|GetL_ImpactLocation) 0 0 "10.000000,10.000000,70.000000"))
            (if (and (Math|Float|NearlyEqual(Float) (.X (Math|Vector|BreakVector (.ProjectedLocation (AI|Navigation|ProjectPointtoNavigation (LocalVariables|GetL_ImpactLocation) 0 0 "10.000000,10.000000,70.000000")))) (.X (Math|Vector|BreakVector (Utilities|Array|Get(acopy) (Variables|/Script/Engine.NavigationPath|GetPathPoints _returnvalue_2) (Utilities|Array|LastIndex (Variables|/Script/Engine.NavigationPath|GetPathPoints _returnvalue_2))))) 5.0) (Math|Float|NearlyEqual(Float) (.Y (Math|Vector|BreakVector (.ProjectedLocation (AI|Navigation|ProjectPointtoNavigation (LocalVariables|GetL_ImpactLocation) 0 0 "10.000000,10.000000,70.000000")))) (.Y (Math|Vector|BreakVector (Utilities|Array|Get(acopy) (Variables|/Script/Engine.NavigationPath|GetPathPoints _returnvalue_2) (Utilities|Array|LastIndex (Variables|/Script/Engine.NavigationPath|GetPathPoints _returnvalue_2))))) 5.0))
              (if (Math|Boolean|ORBoolean (not (> (* (.Roll (Math|Rotator|BreakRotator (LocalVariables|GetL_NormalRotation))) -1.0) 45.0)) (not (> (* (.Pitch (Math|Rotator|BreakRotator (LocalVariables|GetL_NormalRotation))) -1.0) -45.0)) (not (> (* (.Yaw (Math|Rotator|BreakRotator (LocalVariables|GetL_NormalRotation))) -1.0) -45.0)))
                (bind _returnvalue_3 (Collision|SphereTraceForObjects (+ (LocalVariables|GetL_ImpactLocation) "0, 0,15.000000") (+ (LocalVariables|GetL_ImpactLocation) "0, 0,15.000000") 1e+01 (Utilities|Array|MakeArray "ObjectTypeQuery1") false 0 "None"))
                (if _returnvalue_3
                  (Development|PrintString "block")
                  (else
                    (Class|InstancedStaticMeshComponent|AddInstanceWorldSpace (Variables|Default|GetMasterInstance) (Math|Transform|MakeTransform (LocalVariables|GetL_ImpactLocation) (LocalVariables|GetL_NormalRotation) World%20Transform%20Scale))
                    (Utilities|Array|Add (Variables|Default|GetArrayHexGridLocation) (LocalVariables|GetL_ImpactLocation))))))))))
    (:Completed
      (for _array_element_2 (LocalVariables|GetL_ArrayOutHits)
        (if (Utilities|Array|ContainsItem (Variables|Default|GetArrayHexGridLocation) (Math|Vector|MakeVector 0.0 0.0 (.z (.ImpactPoint (Collision|BreakHitResult _array_element_2)))))
          _)))))